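; BPC_SinasoidalMovement is a component that bobs its owning actor up and down along world Z in a sine wave.
; Each tick it adds the change in sine of accumulated time, multiplied by SinasoidalScale, to the actor's current height, leaving X and Y unchanged.
; Because the offset is incremental, the motion needs no stored start position and builds on whatever location the actor currently has.
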(event EventTick
  (params (DeltaSeconds :type Float%20%28single-precision%29))
  (bind _returnvalue (Components|GetOwner))
  (bind _returnvalue_2 (Transformation|GetActorLocation _returnvalue))
  (Variables|Default|SetDeltaTime DeltaSeconds)
  (Transformation|SetActorLocation _returnvalue (Math|Vector|MakeVector (.x _returnvalue_2) (.y _returnvalue_2) (+ (* (- (Math|Trig|Sin(Radians) (+ (Variables|Default|GetDeltaTime) (Variables|Default|GetTotalTime))) (Math|Trig|Sin(Radians) (Variables|Default|GetTotalTime))) (Variables|Default|GetSinasoidalScale)) (.z _returnvalue_2))) false)
  (Variables|Default|SetTotalTime (+ (Variables|Default|GetDeltaTime) (Variables|Default|GetTotalTime))))

(event EventInitializeComponent)