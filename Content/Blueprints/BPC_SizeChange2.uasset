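; Actor component that makes its owning actor pulse in size uniformly over time.
; Each tick it adds the change in a sine wave since the last frame, multiplied by SinasoidalScale, to all three axes of the owner's current scale.
; Accumulated TotalTime drives the wave, and this incremental approach oscillates around the existing scale without storing a base value.
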(event Custom|ReceiveInitializeComponent_Copy)

(event EventTick
  (params (DeltaSeconds :type Float%20%28single-precision%29))
  (bind _returnvalue (Components|GetOwner))
  (bind _returnvalue_2 (Transformation|GetActorScale3D _returnvalue))
  (Variables|Default|SetDeltaTime DeltaSeconds)
  (Transformation|SetActorScale3D _returnvalue (Math|Vector|MakeVector (+ (* (- (Math|Trig|Sin(Radians) (+ (Variables|Default|GetDeltaTime) (Variables|Default|GetTotalTime))) (Math|Trig|Sin(Radians) (Variables|Default|GetTotalTime))) (Variables|Default|GetSinasoidalScale)) (.x _returnvalue_2)) (+ (* (- (Math|Trig|Sin(Radians) (+ (Variables|Default|GetDeltaTime) (Variables|Default|GetTotalTime))) (Math|Trig|Sin(Radians) (Variables|Default|GetTotalTime))) (Variables|Default|GetSinasoidalScale)) (.y _returnvalue_2)) (+ (* (- (Math|Trig|Sin(Radians) (+ (Variables|Default|GetDeltaTime) (Variables|Default|GetTotalTime))) (Math|Trig|Sin(Radians) (Variables|Default|GetTotalTime))) (Variables|Default|GetSinasoidalScale)) (.z _returnvalue_2))))
  (Variables|Default|SetTotalTime (+ (Variables|Default|GetDeltaTime) (Variables|Default|GetTotalTime))))

(event EventInitializeComponent)