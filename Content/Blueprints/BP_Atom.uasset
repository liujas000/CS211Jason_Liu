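; BP_Atom is an actor that acts as a proton or as an electron orbiting a Parent actor.
; The construction script applies the electron material when Parent is valid, otherwise the proton material.
; Each Tick, an instance with a Parent rotates its offset around that actor by Pitch, Rotation and Yaw scaled by Speed, without delta time, so orbit speed depends on frame rate.
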(event EventBeginPlay)

(event EventActorBeginOverlap
  (params (OtherActor :type Actor%20Object%20Reference)))

(event EventTick
  (params (DeltaSeconds :type Float%20%28single-precision%29))
  (bind _parent (Variables|Default|GetParent))
  (bind _speed (Variables|Default|GetSpeed))
  (bind _returnvalue (Transformation|GetActorLocation _parent))
  (Utilities|IsValid (Variables|Default|GetParent)
    (:Is%20Valid
      (Transformation|SetActorLocation (+ (Math|Vector|RotateVector (- (Transformation|GetActorLocation) _returnvalue) (Math|Rotator|MakeRotator (* (Variables|Default|GetPitch) _speed) (* (Variables|Default|GetRotation) _speed) (* (Variables|Default|GetYaw) _speed))) _returnvalue) false))))

(fn ConstructionScript
  (Utilities|IsValid (Variables|Default|GetParent)
    (:Is%20Valid
      (Rendering|Material|SetMaterial 0 (Variables|Default|GetMaterial_Electron)))
    (:Is%20Not%20Valid
      (Rendering|Material|SetMaterial 0 (Variables|Default|GetMaterial_Proton)))))