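; BP_CelestialBody is an actor that orbits a Parent actor around the vertical axis.
; Each tick, while Parent is valid, it rotates its current offset from Parent in yaw and sets its location without sweep.
; The yaw step is Rotation divided by the square root of the distance, so farther bodies orbit more slowly.
; The step is not scaled by delta time, making orbit speed frame-rate dependent.
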(event EventBeginPlay)

(event EventActorBeginOverlap
  (params (OtherActor :type Actor%20Object%20Reference)))

(event EventTick
  (params (DeltaSeconds :type Float%20%28single-precision%29))
  (bind _returnvalue (Transformation|GetActorLocation))
  (bind _parent (Variables|Default|GetParent))
  (bind _returnvalue_2 (Transformation|GetActorLocation _parent))
  (Utilities|IsValid (Variables|Default|GetParent)
    (:Is%20Valid
      (Transformation|SetActorLocation (+ (Math|Vector|RotateVector (- _returnvalue _returnvalue_2) (Math|Rotator|MakeRotator 0.0 (/ (Variables|Default|GetRotation) (Math|Float|Sqrt (Math|Vector|VectorLength (- _returnvalue_2 _returnvalue)))) 0.0)) _returnvalue_2) false))))

(fn ConstructionScript)