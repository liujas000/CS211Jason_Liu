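; BP_ColumnRow is an actor that builds a row of wooden static mesh columns toward an EndPoint vector.
; Its construction script runs only when EndPoint has a non-zero X, adding one BrownWood mesh every 60 units along the vector's length.
; The meshes attach along the Column component's local X axis, and Column rotates to face the actor location plus EndPoint.
; The event graph holds no logic.
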(event EventBeginPlay)

(event EventActorBeginOverlap
  (params (OtherActor :type Actor%20Object%20Reference)))

(event EventTick
  (params (DeltaSeconds :type Float%20%28single-precision%29)))

(fn ConstructionScript
  (bind _returnvalue (Transformation|GetActorLocation))
  (if (Math|Vector|NotEqual(Vector) (* (Variables|Default|GetEndPoint) "1.000000,0.000000,0.000000") "0, 0, 0" 0.0)
    (for _index (range 1 (Math|Float|Floor (/ (Math|Vector|VectorLength (Variables|Default|GetEndPoint)) 6e+01)))
      (bind _returnvalue_2 (AddComponent|AddStaticMeshComponent true))
      (Rendering|Material|SetMaterial _returnvalue_2 0 "/Game/NewSarterContent/Material/BrownWood.BrownWood")
      (Class|SceneComponent|Attachto _returnvalue_2 (Variables|Default|GetColumn) "None" "KeepRelativeOffset" true)
      (Transformation|SetRelativeLocation _returnvalue_2 (Math|Vector|MakeVector (* _index 6e+01) 0.0 0.0) false)
      (Transformation|SetRelativeRotation (Variables|Default|GetColumn) (Math|Rotator|FindLookatRotation _returnvalue (+ _returnvalue (Variables|Default|GetEndPoint))) false))))