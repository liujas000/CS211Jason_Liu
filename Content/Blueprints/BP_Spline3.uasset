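; BP_Spline3 is a construction-script tool that places copies of a static mesh along a spline, with no active event logic.
; It adds a mesh component every LengthInterval units, matching the spline's rotation and applying a uniform Scale.
; The copies cycle through three materials on element 0 by index.
; Spline world-space location and rotation are fed into each component's relative transform.
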(event EventBeginPlay)

(event EventActorBeginOverlap
  (params (OtherActor :type Actor%20Object%20Reference)))

(event EventTick
  (params (DeltaSeconds :type Float%20%28single-precision%29)))

(fn ConstructionScript
  (for _index (range 0 (Math|Float|Floor (/ (Spline|GetSplineLength) (Variables|Default|GetLengthInterval))))
    (bind _returnvalue (AddComponent|AddStaticMeshComponent false))
    (Transformation|SetRelativeTransform _returnvalue (Math|Transform|MakeTransform (Class|SplineComponent|GetWorldLocationatDistanceAlongSpline (* _index (Variables|Default|GetLengthInterval))) (Class|SplineComponent|GetWorldRotationatDistanceAlongSpline (* _index (Variables|Default|GetLengthInterval))) (Math|Conversions|ToVector(Float) (Variables|Default|GetScale))) false)
    (Components|StaticMesh|SetStaticMesh _returnvalue (Variables|Default|GetMesh))
    (switch int (Math|Integer|%(Integer) _index 3)
      (:0
        (Rendering|Material|SetMaterial _returnvalue 0 (Variables|Default|GetMaterial_1)))
      (:1
        (Rendering|Material|SetMaterial _returnvalue 0 (Variables|Default|GetMaterial_2)))
      (:2
        (Rendering|Material|SetMaterial _returnvalue 0 (Variables|Default|GetMaterial_3))))))