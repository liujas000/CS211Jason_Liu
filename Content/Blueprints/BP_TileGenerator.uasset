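; BP_TileGenerator is a construction-script actor that fills an area from its root to an editable EndPoint with a grid of static mesh tiles.
; Nested loops derive row and column counts from EndPoint, Scale and Space, adding a mesh component per cell.
; Each tile gets uniform scale, a shared material, and random height and rotation offsets, re-rolled whenever construction reruns.
; Event graph logic is empty.
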(event EventBeginPlay)

(event EventActorBeginOverlap
  (params (OtherActor :type Actor%20Object%20Reference)))

(event EventTick
  (params (DeltaSeconds :type Float%20%28single-precision%29)))

(fn ConstructionScript
  (bind _randheightscale (Variables|Default|GetRandHeightScale))
  (bind _randrotationscale (Variables|Default|GetRandRotationScale))
  (bind _space (Variables|Default|GetSpace))
  (bind _scale (Variables|Default|GetScale))
  (bind _returnvalue (* _scale 1e+02))
  (bind _returnvalue_2 (+ _space _returnvalue))
  (for _index (range 0 (Math|Float|Floor (/ (.y (Variables|Default|GetEndPoint)) _returnvalue_2)))
    (for _index_2 (range 0 (Math|Float|Floor (/ (.x (Variables|Default|GetEndPoint)) _returnvalue_2)))
      (bind _returnvalue_3 (AddComponent|AddStaticMeshComponent true))
      (Class|SceneComponent|Attachto _returnvalue_3 (Variables|Default|GetRoot) "None" "KeepRelativeOffset" true)
      (Transformation|SetRelativeLocation _returnvalue_3 (Math|Vector|MakeVector (* _index_2 _returnvalue_2) (* _index _returnvalue_2) (Math|Random|RandomFloatinRange (* _randheightscale -1.0) _randheightscale)) false)
      (Transformation|SetRelativeScale3D _returnvalue_3 (Math|Conversions|ToVector(Float) (Variables|Default|GetScale)))
      (Transformation|SetRelativeRotation _returnvalue_3 (Math|Rotator|MakeRotator (Math|Random|RandomFloatinRange 0.0 _randrotationscale) (Math|Random|RandomFloatinRange 0.0 _randrotationscale) (Math|Random|RandomFloatinRange 0.0 _randrotationscale)) false)
      (Rendering|Material|SetMaterial _returnvalue_3 0 (Variables|Default|GetMaterial)))))